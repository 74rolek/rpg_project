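; BP_CheetZ_menager is a cheat manager Blueprint with functions to grant XP, set god mode and teleport the player.
; XP and god mode go through GameInstance_MOJ, calling DodajXP or setting the GodMode flag, which is printed to screen.
; Teleport runs a debug-drawn vertical Visibility trace at the given X/Y and moves the player pawn to the hit location, without checking that it hit.
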(fn //giveXP
  (params (xp :type Integer))
  (bind _asgame_instance_moj (Utilities|Casting|CastToGameInstance_MOJ (Game|GetGameInstance)))
  (bind _output_get (Variables|Default|SetAs%20Game%20Instance%20MOJ _asgame_instance_moj))
  (Class|GameInstanceMOJ|DodajXP _output_get xp))

(fn //gameModeGod
  (params (God%20Mode :type Boolean))
  (bind _asgame_instance_moj (Utilities|Casting|CastToGameInstance_MOJ (Game|GetGameInstance)))
  (bind _output_get (Variables|Default|SetAs%20Game%20Instance%20MOJ _asgame_instance_moj))
  (bind _output_get_2 (Variables|/Script/EldenRings.GameInstance_MOJ|SetGodMode _output_get God%20Mode))
  (Development|PrintString (Utilities|String|ToString(Text) (Utilities|Text|FormatText "GodMode {valuel}" _output_get_2))))

(fn //teleport
  (params (Połozenie%20Y :type Integer) (Położenie%20X :type Integer))
  (bind _returnvalue (Math|Conversions|ToFloat(Integer) Połozenie%20Y))
  (bind _returnvalue_2 (Math|Conversions|ToFloat(Integer) Położenie%20X))
  (bind _outhit (Collision|LineTraceByChannel (Math|Vector|MakeVector _returnvalue_2 _returnvalue 1e+05) (Math|Vector|MakeVector _returnvalue_2 _returnvalue -1e+05) "TraceTypeQuery1" false 0 "ForDuration"))
  (Transformation|SetActorLocation (Game|Player|GetPlayerPawn 0) (.Location (Collision|BreakHitResult _outhit)) false false))