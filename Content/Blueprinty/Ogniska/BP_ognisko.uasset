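; BP_ognisko is a campfire actor that the player can interact with to open the campfire screen in the HUD.
; Its prompt widget starts hidden and is shown or hidden through SetSelected.
; Every Tick it rotates its Scene component to face the player pawn.
; Interact casts the interactor to BP_ThirdPersonCharacter and calls the CEOtwórzOgnisko event on that character's HUD widget.
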(event EventBeginPlay
  (Rendering|SetVisibility (Variables|Default|GetWidget) false false))

(event Collision|EventActorBeginOverlap
  (params (OtherActor :type Actor%20Object%20Reference)))

(event EventTick
  (params (DeltaSeconds :type Float%20%28single-precision%29))
  (bind _scene (Variables|Default|GetScene))
  (Transformation|SetWorldRotation _scene (Math|Rotator|FindLookatRotation (Transformation|GetWorldLocation _scene) (Transformation|GetActorLocation (Game|Player|GetPlayerPawn 0))) false false))

(event EventInteract
  (params (Interactor :type Actor%20Object%20Reference))
  (bind _asbp_third_person_character (Utilities|Casting|CastToBP_ThirdPersonCharacter Interactor))
  (Default|CEOtwórzOgnisko (Variables|/Game/ThirdPerson/Blueprints/BP_ThirdPersonCharacter.BP_ThirdPersonCharacter_C|GetAs%20WB+Hudd _asbp_third_person_character)))

(event EventSetSelected
  (params (bIsSelected :type Boolean))
  (Rendering|SetVisibility (Variables|Default|GetWidget) bIsSelected false))

(fn ConstructionScript)